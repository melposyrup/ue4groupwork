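; Test player controller, kept in the Ending folder, that routes basic movement, look and jump input to the player character.
; Jump press and release start and stop jumping on player character 0, and move axes add movement along the controller's own forward and right vectors.
; Turn and LookUp axes feed the controller's yaw and pitch.
; A Debug action only prints a placeholder greeting.
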(event `InputAction|Jump`
  (params (Key :type "Key Structure"))
  (bind _returnvalue (`GameplayStatics.GetPlayerCharacter` 0))
  ;[1 1 1] Input Jump
  (:`Pressed`
    (`Character.Jump` _returnvalue))
  (:`Released`
    (`Character.StopJumping` _returnvalue)))

(event `InputAxis|MoveForward`
  (params (AxisValue :type "Float (single-precision)"))
  ;[1 1 1] Input Move
  (`Pawn.AddMovementInput` (`GameplayStatics.GetPlayerCharacter` 0) (`self.GetActorForwardVector`) AxisValue false))

(event `InputAxis|MoveRight`
  (params (AxisValue :type "Float (single-precision)"))
  ;[1 1 1] Input Move
  (`Pawn.AddMovementInput` (`GameplayStatics.GetPlayerCharacter` 0) (`self.GetActorRightVector`) AxisValue false))

(event `InputAxis|Turn`
  (params (AxisValue :type "Float (single-precision)"))
  ;[1 1 1] Input View
  (`self.AddYawInput` AxisValue))

(event `InputAxis|LookUp`
  (params (AxisValue :type "Float (single-precision)"))
  ;[1 1 1] Input View
  (`self.AddPitchInput` AxisValue))

(event `InputAction|Debug`
  (params (Key :type "Key Structure"))
  (:`Pressed`
    (`KismetSystemLibrary.PrintString` "Hello")))

(fn `UserConstructionScript`)