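; Input controller Blueprint that detects whether the player is using a gamepad or keyboard and mouse, intended to drive tutorial sprite display.
; Gamepad stick and mouse axis events above a small dead zone flip IsKeyboard only on a change, then fire OnInputDeviceChanged with the new state.
; Debug prints show each switch, and a TEST input action opens the Ending level.
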(event `InputAction|TEST`
  (params (Key :type "Key Structure"))
  (:`Pressed`
    (`GameplayStatics.OpenLevelBySoftObjectPtr` "/Game/k0214/Maps/Ending.Ending")))

(event `InputVectorAxis|Gamepad_Left2D`
  (params (AxisValue :type "Vector Structure"))
  ;[1 1 1] Gamepad(controller) trigger for tutorialSpriteDisplay
  (`self.CallOnController` AxisValue))

(event `InputVectorAxis|Gamepad_Right2D`
  (params (AxisValue :type "Vector Structure"))
  ;[1 1 1] Gamepad(controller) trigger for tutorialSpriteDisplay
  (`self.CallOnController` AxisValue))

(event `InputVectorAxis|Mouse2D`
  (params (AxisValue :type "Vector Structure"))
  ;[1 1 1] Keyboard trigger
  (`self.CallOnKeyboard` AxisValue))

(fn `CallOnController`
  (params (A :type "Vector Structure"))
  (if (> (`KismetMathLibrary.VSize` A) 0.1)
    (if (`self.IsKeyboard`)
      (bind _output_get (set `self.IsKeyboard` false))
      (`KismetSystemLibrary.PrintString` "controller" true false (struct :`G` 0.66 :`B` 1.0 :`A` 1.0) 0.0)
      (`self.OnInputDeviceChanged` _output_get))))

(fn `CallOnKeyboard`
  (params (A :type "Vector Structure"))
  (if (> (`KismetMathLibrary.VSize` A) 0.1)
    (if (not (`self.IsKeyboard`))
      (bind _output_get (set `self.IsKeyboard` true))
      (`KismetSystemLibrary.PrintString` "keyboard" true false (struct :`R` 1.0 :`G` 0.026767 :`A` 1.0) 0.0)
      (`self.OnInputDeviceChanged` _output_get))))

(fn `UserConstructionScript`)