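; Player character Blueprint for the neko player, handling stick movement, sprint, interaction and a debug return to the Title level.
; Sprint input drives StaminaComponent, whose state selects walk or sprint speed whenever computed stick magnitude is outside the partial-tilt range.
; Interact messages HitInteractiveActor and passes the result on as an objective ID, but the trace that sets that actor is disconnected.
; BeginPlay spawns a test map UI root actor.
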(event `self.ReceiveBeginPlay`
  ;[1 1 1] TEST: Create MapUI root actor
  (bind _returnvalue (`|SpawnActorFromClass` "/Game/k0214/Blueprints/BP_MapRootActor.BP_MapRootActor_C" (`KismetMathLibrary.Conv_VectorToTransform` (`self.K2_GetActorLocation` (`/Game/k0214/Blueprints/CommonFunctionLibrary.GetPlayer`))) "AlwaysSpawn" "OverrideRootScale" null null))
  (set `self.MapUIActor` _returnvalue))

(event `InputAction|Sprint`
  (params (Key :type "Key Structure"))
  (bind _staminacomponent (`self.StaminaComponent`))
  ;[1 1 1] Sprint
  (:`Pressed`
    (`/Game/k0214/Blueprints/StaminaComponent.StartSprint` _staminacomponent))
  (:`Released`
    (`/Game/k0214/Blueprints/StaminaComponent.StopSprint` _staminacomponent)))

(event `InputAction|Interact`
  (params (Key :type "Key Structure"))
  (bind _hitinteractiveactor (`self.HitInteractiveActor`))
  (:`Pressed`
    (`GameplayStatics.PlaySound2D` "/Game/k0214/Assets/Sound/interactSE.interactSE" 1.0 1.0 0.0 null null)
    ;[1 1 1] Press F for Interaction
    (`/Engine/EditorBlueprintResources/StandardMacros.IsValid` _hitinteractiveactor
      (:`Is Valid`
        (bind _objetiveid (message `/Game/k0214/Blueprints/I_Interaction.InteractionImplement` _hitinteractiveactor))
        (`self.OnObjectiveIDCalled` _objetiveid)
        (`KismetSystemLibrary.PrintString` (`KismetSystemLibrary.GetDisplayName` (`self.HitInteractiveActor`)) true true (struct :`G` 0.66 :`B` 1.0 :`A` 1.0) 10.0)))))

(event `InputAction|Debug`
  (params (Key :type "Key Structure"))
  (:`Pressed`
    (`GameplayStatics.OpenLevelBySoftObjectPtr` "/Game/k0214/Maps/Title.Title")))

(event `InputAxis|MoveForward`
  (params (AxisValue :type "Float (single-precision)"))
  (bind _charactermovement (`self.CharacterMovement`))
  ;[1 1 1] Controller LeftStick dynamic input
  (bind _output_get (set `self.ForwardAxis` AxisValue))
  (set `self.F_Axis` (`self.CalculateAxis`))
  (`self.AddMovementInput` (`self.GetVector`) _output_get)
  (if (`self.GetMaxInput` (`self.MovementChange`)) :!label _label
    _
    (elif (`/Game/k0214/Blueprints/StaminaComponent.IsSptint` (`self.StaminaComponent`))
      (set `CharacterMovementComponent.MaxWalkSpeed` 600.0 _charactermovement)
      (set `CharacterMovementComponent.MinAnalogWalkSpeed` 600.0 _charactermovement)
      (`KismetSystemLibrary.PrintString` "sprint" true true (struct :`G` 0.66 :`B` 1.0 :`A` 1.0) 0.0)
      (else
        (set `CharacterMovementComponent.MaxWalkSpeed` 300.0 _charactermovement)
        (set `CharacterMovementComponent.MinAnalogWalkSpeed` 300.0 _charactermovement)
        (`KismetSystemLibrary.PrintString` "walk" true true (struct :`G` 0.66 :`B` 1.0 :`A` 1.0) 0.0)))))

(event `InputAxis|MoveRight`
  (params (AxisValue :type "Float (single-precision)"))
  ;[1 1 1] Controller LeftStick dynamic input
  (bind _output_get (set `self.RightAxis` AxisValue))
  (set `self.R_Axis` (`.R_Axis` (`self.CalculateAxis`)))
  (`self.AddMovementInput` (`.Right` (`self.GetVector`)) _output_get)
  (goto _label))

(fn `CalculateAxis`
  (returns (F_Axis :type "Float (double-precision)") (R_Axis :type "Float (double-precision)"))
  (bind _returnvalue (`KismetMathLibrary.DegAtan2` (`self.ForwardAxis`) (`self.RightAxis`)))
  (return (/ (`self.ForwardAxis`) (`KismetMathLibrary.DegSin` _returnvalue)) (/ (`self.RightAxis`) (`KismetMathLibrary.DegCos` _returnvalue))))

(fn `CheckMainQuestName`
  (params (QuestName :type Name))
  (returns (IsNextMainQuest :type Boolean))
  (return (== (`KismetStringLibrary.Conv_StringToInt` (`KismetTextLibrary.Conv_TextToString` (`KismetTextLibrary.Conv_NameToText` QuestName))) (`/Game/k0214/QuestSystem/QuestLogComponent.MainQuestProgress` (`self.QuestLogComponent`)))))

(fn `GetMaxInput`
  (params (Movement_Change :type "Float (double-precision)"))
  (returns (ReturnValue :type Boolean))
  (bind _f_axis (`self.F_Axis`))
  (bind _r_axis (`self.R_Axis`))
  (return (or (and (> _f_axis 0.0) (< _f_axis Movement_Change)) (and (> _r_axis 0.0) (< _r_axis Movement_Change)))))

(fn `Interact UI Check`
  (returns (CanInteract :type Boolean))
  (bind _viewcamera (`self.ViewCamera`))
  (bind _returnvalue (`SceneComponent.K2_GetComponentLocation` _viewcamera))
  (bind (_outhit _returnvalue_2) (`KismetSystemLibrary.LineTraceSingle` _returnvalue (+ _returnvalue (* (`SceneComponent.GetForwardVector` _viewcamera) 600.0)) "TraceTypeQuery2"))
  (if _returnvalue_2
    (bind (_bblockinghit _binitialoverlap _time _distance _location _impactpoint _normal _impactnormal _physmat _hitactor) (`GameplayStatics.BreakHitResult` _outhit))
    (if (`KismetSystemLibrary.DoesImplementInterface` _hitactor "/Game/k0214/Blueprints/I_Interaction.I_Interaction_C")
      (cast `/Game/k0214/Blueprints/Enemy/BP_Enemy` _hitactor
        (:`then`
          (return false))
        (:`CastFailed`
          (return true)))
      (else
        (return false)))
    (else
      (return false))))

(fn `InteractionRaytrace`
  ;[1 1 1] save interactive actor to HitInteractiveActor
)

(fn `UserConstructionScript`)