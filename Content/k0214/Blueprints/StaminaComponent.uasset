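; Player stamina component for sprinting, left mostly disconnected, so in its current state it only tracks sprint and recovery flags.
; BeginPlay caches the player's CharacterMovement and derives the recovery rate from sprint cost.
; StartSprint sets the sprint flag if stamina remains, and StopSprint clears it.
; Tick is empty: stamina drain, delayed regeneration, walk-speed scaling and overlay icon toggling never run, and the clamped stamina calculations are unused.
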(event `self.ReceiveBeginPlay`
  (set `self.Character Movement` (`Character.CharacterMovement` (`/Game/k0214/Blueprints/CommonFunctionLibrary.GetPlayer`)))
  (set `self.SprinRecover` (* (`self.SprintCost`) 2.0)))

(event `self.ReceiveTick`
  (params (DeltaSeconds :type "Float (single-precision)")))

(fn `StartSprint`
  (if (> (`self.Stamina`) 0.0)
    (set `self.IsSptint` true)
    (set `self.IsRecovery` false)))

(fn `StopSprint`
  (if (`self.IsSptint`)
    (set `self.IsSptint` false)))