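; BP_HeadGear is a collectible hat pickup that BP_NekoPlayer wears on touching it.
; It spins by a fixed local rotation each Tick, not scaled by delta time.
; On Sphere overlap it copies its mesh to the player's PlayerHeadGear and plays a quest-complete sound.
; It then increments HatNum on GI_test and destroys itself, only if that game instance cast succeeds.
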(event `self.ReceiveTick`
  (params (DeltaSeconds :type "Float (single-precision)"))
  (`self.K2_AddActorLocalRotation` (struct :`Yaw` 3.0)))

(event `self.Sphere.OnComponentBeginOverlap`
  (params (OverlappedComponent :type "PrimitiveComponent Object Reference") (OtherActor :type "Actor Object Reference") (OtherComp :type "PrimitiveComponent Object Reference") (OtherBodyIndex :type Integer) (bFromSweep :type Boolean) (SweepResult :type "HitResult Structure (by ref)"))
  (bind _asbp_neko_player (cast `/Game/k0214/Blueprints/BP_NekoPlayer` OtherActor))
  (`StaticMeshComponent.SetStaticMesh` (`/Game/k0214/Blueprints/BP_NekoPlayer.PlayerHeadGear` _asbp_neko_player) (`StaticMeshComponent.StaticMesh` (`self.StaticMesh`)))
  (`GameplayStatics.PlaySound2D` "/Game/k0214/Assets/Sound/questCompleteSE.questCompleteSE" 1.0 1.0 0.0 null null)
  ;[1 1 1] test game instance
  (bind _asgi_test (cast `/Game/test/GI_test` (`GameplayStatics.GetGameInstance`)))
  (set `/Game/test/GI_test.HatNum` (+ (`/Game/test/GI_test.HatNum` _asgi_test) 1) _asgi_test)
  (`self.K2_DestroyActor`))

(fn `UserConstructionScript`)