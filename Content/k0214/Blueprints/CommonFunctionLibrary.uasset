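; Blueprint function library of shared helpers for the Neko game's player, game mode, HUD overlay and objective markers.
; Getter functions cast the first player's character, the game mode and the HUD's overlay widget to their Neko-specific classes.
; ShowObjectiveIcon scans every NPC_Target actor and sets icon visibility on those whose ObjectiveID matches the given one.
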(fn `GetGameMode`
  (returns (GameMode :type "/Game/k0214/Blueprints/BP_NekoGameMode Object Reference"))
  (bind _asbp_neko_game_mode (cast `/Game/k0214/Blueprints/BP_NekoGameMode` (`GameplayStatics.GetGameMode` null)))
  (return _asbp_neko_game_mode))

(fn `GetPlayer`
  (returns (Player :type "/Game/k0214/Blueprints/BP_NekoPlayer Object Reference"))
  (bind _asbp_neko_player (cast `/Game/k0214/Blueprints/BP_NekoPlayer` (`GameplayStatics.GetPlayerCharacter` null)))
  (return _asbp_neko_player))

(fn `GetPlayerOverlay`
  (returns (NekoOverlay :type "/Game/k0214/Blueprints/WBP_NekoOverlay Object Reference"))
  (bind _asbp_neko_hud (cast `/Game/k0214/Blueprints/BP_NekoHUD` (`PlayerController.GetHUD` (`GameplayStatics.GetPlayerController` null))))
  (bind _aswbp_neko_overlay (cast `/Game/k0214/Blueprints/WBP_NekoOverlay` (`NekoHUD.GetNekoOverlay` _asbp_neko_hud)))
  (return _aswbp_neko_overlay))

(fn `Show Objective Icon`
  (params (ObjectiveID :type String) (Visible :type Boolean))
  (bind _outactors (`GameplayStatics.GetAllActorsOfClass` null "/Game/k0214/QuestSystem/NPC_Target.NPC_Target_C"))
  (for _array_element _outactors
    (if (`KismetStringLibrary.EqualEqual_StrStr` (`/Game/k0214/QuestSystem/NPC_Target.ObjectiveID` _array_element) (`local.ObjectiveID`))
      (`/Game/k0214/QuestSystem/NPC_Target.SetIconVisiblity` _array_element (`local.Visible`)))))