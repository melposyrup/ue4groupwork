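; Spline loop Blueprint that moves a referenced actor endlessly along a spline at constant speed, facing the direction of travel.
; BeginPlay scales the timeline rate by Speed over spline length, then each update maps the track to distance, setting location and tangent-based rotation, and replays on finish.
; The construction script positions the actor at DistanceStart using local-space coordinates.
; An uncalled SplineTransform function wraps distance but returns the transform at zero.
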(event `self.ReceiveBeginPlay`
  (`TimelineComponent.SetPlayRate` (`self.Timeline_0`) (/ (`self.speed`) (`SplineComponent.GetSplineLength` (`self.Spline`))))
  (`self.Play timeline`))

(event `Play timeline`
  (bind _spline (`self.Spline`))
  (bind _spline_2 (`self.Spline`))
  (bind _actor (`self.actor`))
  (bind (_direction _newtrack_0) (`Timeline|Timeline_0` :!via `PlayFromStart`)
    (:`Update`
      (bind _returnvalue (`KismetMathLibrary.Lerp` 0.0 (`SplineComponent.GetDistanceAlongSplineAtSplinePoint` _spline (- (`SplineComponent.GetNumberOfSplinePoints` _spline) 1)) _newtrack_0))
      (`self.K2_SetActorLocation` _actor (`SplineComponent.GetLocationAtDistanceAlongSpline` _spline_2 _returnvalue "World") false false)
      (`self.K2_SetActorRotation` _actor (`KismetMathLibrary.Conv_VectorToRotator` (`SplineComponent.GetTangentAtDistanceAlongSpline` _spline_2 _returnvalue "World")) false))
    (:`Finished`
      (`self.Play timeline`))))

(fn `splineTransform`
  (params (distance :type "Float (double-precision) (by ref)") (speed :type "Float (double-precision)"))
  (returns (transform :type "Transform Structure"))
  (`|VariableSetRef` distance (`KismetMathLibrary.FWrap` (+ distance speed) 0.0 (`SplineComponent.GetSplineLength` (`self.Spline`))))
  (return (`SplineComponent.GetTransformAtDistanceAlongSpline` (`self.Spline`) 0.0 "World" false)))

(fn `UserConstructionScript`
  (`self.K2_SetActorLocation` (`self.actor`) (`SplineComponent.GetLocationAtDistanceAlongSpline` (`self.Spline`) (`self.distanceStart`) "Local") false false))