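; Tutorial prompt actor that shows either a keyboard or a controller Paper2D sprite to match the player's input device.
; On BeginPlay it shows the keyboard sprite and binds to BP_Controller's OnInputDeviceChanged dispatcher.
; Device changes swap the visible sprite instantly through sprite color alpha.
; A looping timeline cross-fade between the two sprites also exists, but nothing starts it.
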(event `self.ReceiveBeginPlay`
  ;[1 1 1] show Keyboard as default
  (`PaperSpriteComponent.SetSpriteColor` (`self.PaperSprite_keyboard`) (make `LinearColor` 1.0 1.0 1.0 1.0))
  (`PaperSpriteComponent.SetSpriteColor` (`self.PaperSprite_controller`) (make `LinearColor` 1.0 1.0 1.0))
  ;[1 1 1] listen to the event dispatcher
  (bind _asbp_controller (cast `/Game/k0214/Blueprints/Ending/BP_Controller` (`GameplayStatics.GetPlayerController` 0)))
  (add `/Game/k0214/Blueprints/Ending/BP_Controller.OnInputDeviceChanged` _asbp_controller (delegate `ChangeTutorialSprite`)))

(event `ChangeTutorialSprite`
  (params (IsKeyboard :type Boolean))
  ;[1 1 1] listen to the event dispatcher
  (if IsKeyboard
    (`self.show keyboard`)
    (else
      (`self.show controller`))))

(event `fadingOut`
  (bind _papersprite_keyboard (`self.PaperSprite_keyboard`))
  (bind _papersprite_controller (`self.PaperSprite_controller`))
  (bind (_spritecolor_r _spritecolor_g _spritecolor_b) (break `LinearColor` (`PaperSpriteComponent.SpriteColor` _papersprite_controller)))
  (bind (_spritecolor_r_2 _spritecolor_g_2 _spritecolor_b_2) (break `LinearColor` (`PaperSpriteComponent.SpriteColor` _papersprite_keyboard)))
  ;[0.2396 0.2396 0.2396] keyboard fading out -> controller fading in
  (bind (_direction _newtrack_0) (`Timeline|TimelineFadingout` :!via `PlayFromStart`)
    (:`Update`
      (`PaperSpriteComponent.SetSpriteColor` _papersprite_keyboard (make `LinearColor` _spritecolor_r_2 _spritecolor_g_2 _spritecolor_b_2 _newtrack_0))
      (`PaperSpriteComponent.SetSpriteColor` _papersprite_controller (make `LinearColor` _spritecolor_r _spritecolor_g _spritecolor_b (- 1.0 _newtrack_0))))
    (:`Finished`
      (`self.fadingIn`))))

(event `fadingIn`
  (bind _papersprite_keyboard (`self.PaperSprite_keyboard`))
  (bind _papersprite_controller (`self.PaperSprite_controller`))
  (bind (_spritecolor_r _spritecolor_g _spritecolor_b) (break `LinearColor` (`PaperSpriteComponent.SpriteColor` _papersprite_keyboard)))
  (bind (_spritecolor_r_2 _spritecolor_g_2 _spritecolor_b_2) (break `LinearColor` (`PaperSpriteComponent.SpriteColor` _papersprite_controller)))
  ;[0.2396 0.2396 0.2396] controller fading out -> keyboard fading in
  (bind (_direction _newtrack_0) (`Timeline|Timeline_0` :!via `ReverseFromEnd`)
    (:`Update`
      (`PaperSpriteComponent.SetSpriteColor` _papersprite_keyboard (make `LinearColor` _spritecolor_r _spritecolor_g _spritecolor_b _newtrack_0))
      (`PaperSpriteComponent.SetSpriteColor` _papersprite_controller (make `LinearColor` _spritecolor_r_2 _spritecolor_g_2 _spritecolor_b_2 (- 1.0 _newtrack_0))))
    (:`Finished`
      (`self.fadingOut`))))

(event `show controller`
  (bind _papersprite_keyboard (`self.PaperSprite_keyboard`))
  (bind _papersprite_controller (`self.PaperSprite_controller`))
  (bind (_spritecolor_r _spritecolor_g _spritecolor_b) (break `LinearColor` (`PaperSpriteComponent.SpriteColor` _papersprite_keyboard)))
  (bind (_spritecolor_r_2 _spritecolor_g_2 _spritecolor_b_2) (break `LinearColor` (`PaperSpriteComponent.SpriteColor` _papersprite_controller)))
  ;[1 1 1] show controller
  (`PaperSpriteComponent.SetSpriteColor` _papersprite_keyboard (make `LinearColor` _spritecolor_r _spritecolor_g _spritecolor_b))
  (`PaperSpriteComponent.SetSpriteColor` _papersprite_controller (make `LinearColor` _spritecolor_r_2 _spritecolor_g_2 _spritecolor_b_2 1.0)))

(event `show keyboard`
  (bind _papersprite_keyboard (`self.PaperSprite_keyboard`))
  (bind _papersprite_controller (`self.PaperSprite_controller`))
  (bind (_spritecolor_r _spritecolor_g _spritecolor_b) (break `LinearColor` (`PaperSpriteComponent.SpriteColor` _papersprite_controller)))
  (bind (_spritecolor_r_2 _spritecolor_g_2 _spritecolor_b_2) (break `LinearColor` (`PaperSpriteComponent.SpriteColor` _papersprite_keyboard)))
  ;[1 1 1] show keyboard
  (`PaperSpriteComponent.SetSpriteColor` _papersprite_keyboard (make `LinearColor` _spritecolor_r_2 _spritecolor_g_2 _spritecolor_b_2 1.0))
  (`PaperSpriteComponent.SetSpriteColor` _papersprite_controller (make `LinearColor` _spritecolor_r _spritecolor_g _spritecolor_b)))

(fn `UserConstructionScript`)