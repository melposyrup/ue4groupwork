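; BP_NekoPlayerController is a player controller that tracks whether keyboard or controller is the active input device and provides debug level shortcuts.
; CallOnController and CallOnKeyboard flip IsKeyboard when the passed vector exceeds a small dead zone, calling CallOnInputDeviceChanged only on an actual switch.
; Each switch also prints the device name on screen.
; Debug F10 and F12 actions open the Title and Ending levels.
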(event `InputAction|DEBUG_F10`
  (params (Key :type "Key Structure"))
  (:`Pressed`
    (`GameplayStatics.OpenLevelBySoftObjectPtr` "/Game/Maps/Title.Title")))

(event `InputAction|DEBUG_F12`
  (params (Key :type "Key Structure"))
  (:`Pressed`
    (`GameplayStatics.OpenLevelBySoftObjectPtr` "/Game/Maps/Ending.Ending")))

(fn `CallOnController`
  (params (A :type "Vector Structure"))
  (if (> (`KismetMathLibrary.VSize` A) 0.1)
    (if (`self.IsKeyboard`)
      (bind _output_get (set `self.IsKeyboard` false))
      (`KismetSystemLibrary.PrintString` "controller" true false (struct :`G` 0.66 :`B` 1.0 :`A` 1.0) 0.0)
      (`self.OnInputDeviceChanged` _output_get))))

(fn `CallOnKeyboard`
  (params (A :type "Vector Structure"))
  (if (> (`KismetMathLibrary.VSize` A) 0.1)
    (if (not (`self.IsKeyboard`))
      (bind _output_get (set `self.IsKeyboard` true))
      (`KismetSystemLibrary.PrintString` "keyboard" true false (struct :`R` 1.0 :`G` 0.026767 :`A` 1.0) 0.0)
      (`self.OnInputDeviceChanged` _output_get))))

(fn `UserConstructionScript`)