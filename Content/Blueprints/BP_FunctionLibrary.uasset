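; Blueprint function library giving Neko game code shortcuts to core objects and toggles for quest markers.
; Getters cast to the game mode, game instance, player character, its quest log component and the HUD overlay.
; The two icon functions scan all NPCs of a class for a matching objective ID or quest row, set icon visibility and update minimap positions.
; Showing an objective also spawns a direction guide actor.
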(fn `GetGameInstance`
  (returns (BP_GameInstance :type "/Game/Blueprints/BP_GameInstance Object Reference"))
  (bind _asbp_game_instance (cast `/Game/Blueprints/BP_GameInstance` (`GameplayStatics.GetGameInstance` null)))
  (return _asbp_game_instance))

(fn `GetGameMode`
  (returns (GameMode :type "/Game/Blueprints/BP_NekoGameModePlay Object Reference"))
  (bind _asbp_neko_game_mode_play (cast `/Game/Blueprints/BP_NekoGameModePlay` (`GameplayStatics.GetGameMode` null)))
  (return _asbp_neko_game_mode_play))

(fn `GetPlayer`
  (returns (Player :type "/Game/Characters/BP_NekoCharacter Object Reference"))
  (bind _asbp_neko_character (cast `/Game/Characters/BP_NekoCharacter` (`GameplayStatics.GetPlayerCharacter` null)))
  (return _asbp_neko_character))

(fn `GetPlayerOverlay`
  (returns (Overlay :type "/Game/Characters/Overlay/WBP_NekoOverlay Object Reference"))
  (bind _asbp_neko_hud (cast `/Game/Blueprints/BP_NekoHUD` (`PlayerController.GetHUD` (`GameplayStatics.GetPlayerController` null))))
  (bind _aswbp_neko_overlay (cast `/Game/Characters/Overlay/WBP_NekoOverlay` (`NekoHUD.GetNekoOverlay` _asbp_neko_hud)))
  (return _aswbp_neko_overlay))

(fn `GetPlayerQuestComp`
  (returns (NewParam :type "/Game/QuestSystem/QuestLogComponent Object Reference"))
  (return (`/Game/Characters/BP_NekoCharacter.QuestLogComponent` (`self.GetPlayer` null))))

(fn `ShowMainQuestIcon`
  (params (visible :type Boolean) (Name :type Name))
  ;[1 1 1] find QuestNPC
  (bind _outactors (`GameplayStatics.GetAllActorsOfClass` null "/Game/QuestSystem/NPC.NPC_C"))
  (for _array_element _outactors
    (bind (_questdata_datatable _questdata_rowname) (break `DataTableRowHandle` (`/Game/QuestSystem/QuestGiverComponent.QuestData` (`/Game/QuestSystem/NPC.QuestGiverComponent` _array_element))))
    (if (== _questdata_rowname Name)
      (if (`local.visible`)
        (`/Game/QuestSystem/NPC.SetIconVisiblity` _array_element true)
        ;[1 1 1] set NPC pos for minimap
        (set `/Game/Characters/Overlay/MinimapUI/WBP_Minimap.QuestPosition` (`Actor.K2_GetActorLocation` _array_element) (`/Game/Characters/Overlay/WBP_NekoOverlay.WBP_Minimap` (`self.GetPlayerOverlay` null)))
        (else
          (`/Game/QuestSystem/NPC.SetIconVisiblity` _array_element false)
          (set `/Game/Characters/Overlay/MinimapUI/WBP_Minimap.QuestPosition` (0.0 0.0 0.0) (`/Game/Characters/Overlay/WBP_NekoOverlay.WBP_Minimap` (`self.GetPlayerOverlay` null))))))))

(fn `ShowObjectiveIcon`
  (params (ObjectiveID :type String) (Visible :type Boolean))
  ;[1 1 1] find TargetNPC
  (bind _outactors (`GameplayStatics.GetAllActorsOfClass` null "/Game/QuestSystem/NPC_Target.NPC_Target_C"))
  (for _array_element _outactors
    (if (`KismetStringLibrary.EqualEqual_StrStr` (`/Game/QuestSystem/NPC_Target.ObjectiveID` _array_element) (`local.ObjectiveID`))
      ;[1 1 1] set visibility of icons in BP_Target and Minimap
      (`/Game/QuestSystem/NPC_Target.SetIconVisiblity` _array_element (`local.Visible`))
      (set `/Game/Characters/Overlay/MinimapUI/WBP_Minimap.TargetPosition` (`/Game/QuestSystem/NPC_Target.GetLocation` _array_element) (`/Game/Characters/Overlay/WBP_NekoOverlay.WBP_Minimap` (`self.GetPlayerOverlay` null)))
      (`SceneComponent.SetVisibility` (`/Game/QuestSystem/NPC_Target.WidgetQuestComplete` _array_element) (`local.Visible`) false)
      ;[1 1 1] if set icon to visible, create BP_Direction as a guide
      (if (`local.Visible`)
        (`/Game/QuestSystem/QuestLogComponent.SpawnTargetDirectionActor` (`self.GetPlayerQuestComp` null) (`Actor.K2_GetActorLocation` _array_element))))))