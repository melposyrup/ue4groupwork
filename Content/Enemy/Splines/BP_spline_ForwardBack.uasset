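; Spline mover Blueprint under Enemy that carries a child actor along a spline path.
; Each Tick advances a distance by Speed and delta time, then copies the spline's local location and rotation at that distance to the child, keeping its scale.
; Despite the ForwardBack name, passing the spline's end resets the distance to zero, so motion restarts from the beginning without reversing.
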(event `self.ReceiveTick`
  (params (DeltaSeconds :type "Float (single-precision)"))
  (bind _returnvalue (`SplineComponent.GetTransformAtDistanceAlongSpline` (`self.Spline`) (`self.distance`) "Local" false))
  (set `self.distance` (+ (* DeltaSeconds (`self.speed`)) (`self.distance`)))
  (if (> (`SplineComponent.GetSplineLength` (`self.Spline`)) (`self.distance`))
    (`SceneComponent.K2_SetRelativeTransform` (`self.ChildActor`) (`KismetMathLibrary.MakeTransform` (`KismetMathLibrary.MakeVector` (.x (.location _returnvalue)) (.y (.location _returnvalue)) (+ (.z (.location _returnvalue)) 0.0)) (`KismetMathLibrary.MakeRotator` (.roll (.rotation _returnvalue)) (.pitch (.rotation _returnvalue)) (+ (.yaw (.rotation _returnvalue)) 0.0)) (`SceneComponent.RelativeScale3D` (`self.ChildActor`))) false false)
    (else
      (set `self.distance` 0.0))))

(fn `UserConstructionScript`)