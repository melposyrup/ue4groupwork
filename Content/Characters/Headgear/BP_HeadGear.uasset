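; BP_HeadGear is a spinning hat pickup for the Neko character.
; On sphere overlap it copies its own static mesh onto the character's PlayerHeadGear component, increases the launch item count and plays a cat sound.
; It then increments the hat counter on the game instance and destroys itself.
; The spin is a fixed rotation applied every tick, not scaled by delta time.
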(event `self.ReceiveTick`
  (params (DeltaSeconds :type "Float (single-precision)"))
  (`SceneComponent.K2_AddLocalRotation` (`self.StaticMesh`) (struct :`Yaw` 3.0) false false))

(event `self.Sphere.OnComponentBeginOverlap`
  (params (OverlappedComponent :type "PrimitiveComponent Object Reference") (OtherActor :type "Actor Object Reference") (OtherComp :type "PrimitiveComponent Object Reference") (OtherBodyIndex :type Integer) (bFromSweep :type Boolean) (SweepResult :type "HitResult Structure (by ref)"))
  ;[1 1 1] add visual to player
  (bind _asbp_neko_character (cast `/Game/Characters/BP_NekoCharacter` OtherActor))
  (`StaticMeshComponent.SetStaticMesh` (`/Game/Characters/BP_NekoCharacter.PlayerHeadGear` _asbp_neko_character) (`StaticMeshComponent.StaticMesh` (`self.StaticMesh`)))
  (`NekoCharacter.LaunchItemCountIncrease` _asbp_neko_character 10)
  (`GameplayStatics.PlaySound2D` "/Game/Sound/cat23_interaction.cat23_interaction" 1.0 1.0 0.0 null null)
  ;[1 1 1] add to game instance
  (`/Engine/EditorBlueprintResources/StandardMacros.IncrementInt` (`/Game/Blueprints/BP_GameInstance.HatNum` (`/Game/Blueprints/BP_FunctionLibrary.GetGameInstance`))
    (:`  `
      (`self.K2_DestroyActor`))))

(fn `UserConstructionScript`)