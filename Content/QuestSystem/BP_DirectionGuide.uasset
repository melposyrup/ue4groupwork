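; BP_DirectionGuide is a quest-system guide actor that follows the player and points toward a target location.
; On BeginPlay it caches the player reference.
; Every Tick it teleports to a fixed height above the player's location, then rotates with a look-at rotation toward TargetLocation, a variable this graph reads but never sets.
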(event `self.ReceiveBeginPlay`
  (set `self.Player` (`/Game/Blueprints/BP_FunctionLibrary.GetPlayer`)))

(event `self.ReceiveTick`
  (params (DeltaSeconds :type "Float (single-precision)"))
  (bind (_returnvalue_roll _returnvalue_pitch _returnvalue_yaw) (`KismetMathLibrary.BreakRotator` (`KismetMathLibrary.FindLookAtRotation` (`self.K2_GetActorLocation`) (`self.targetLocation`))))
  ;[1 1 1] snap to Player
  (`self.K2_SetActorLocation` (+ (`self.K2_GetActorLocation` (`self.Player`)) (0.0 0.0 60.0)) false true)
  ;[1 1 1] point to the target
  (`self.K2_SetActorRotation` (`KismetMathLibrary.MakeRotator` _returnvalue_roll _returnvalue_pitch _returnvalue_yaw)))

(fn `UserConstructionScript`)