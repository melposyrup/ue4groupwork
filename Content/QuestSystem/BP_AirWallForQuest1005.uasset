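; Air wall for Quest 1005 that stays hidden and without collision until that quest starts.
; On BeginPlay it binds to the Quest1005 start event on the player's quest component.
; When the event fires, it shows the mesh, sets the box to block all channels and destroys every BP_spline actor in the world.
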(event `self.ReceiveBeginPlay`
  (`SceneComponent.SetVisibility` (`self.StaticMesh`) false false)
  (`PrimitiveComponent.SetCollisionEnabled` (`self.Box`) "NoCollision")
  (add `/Game/QuestSystem/QuestLogComponent.OnQuest1005Start` (`/Game/Blueprints/BP_FunctionLibrary.GetPlayerQuestComp`) (delegate `SetCollsionToBlockAll`)))

(event `SetCollsionToBlockAll`
  (bind _box (`self.Box`))
  (`|ExecutionSequence`
    (:`then_0`
      ;[1 1 1] Airwall activate
      (`SceneComponent.SetVisibility` (`self.StaticMesh`) true false)
      (`PrimitiveComponent.SetCollisionEnabled` _box "QueryAndPhysics")
      (`PrimitiveComponent.SetCollisionResponseToAllChannels` _box "ECR_Block"))
    (:`then_1`
      (bind _outactors (`GameplayStatics.GetAllActorsOfClass` "/Game/Enemy/Splines/BP_spline.BP_spline_C"))
      (for _array_element _outactors
        (`self.K2_DestroyActor` _array_element)))))

(fn `UserConstructionScript`)